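; Base weapon for the FPS player, handling magazine and reserve ammo, type-matched pickups, reload math and firing.
; StartShooting spends a round, calls AutoReloadOnEmpty on an empty magazine and runs a camera line trace for hitscan, adding random endpoint spread unless aiming.
; Helper checks gate shooting and set the player's CanReload flag.
; The trace only draws debug lines with its hit unused, and AutoReloadOnEmpty holds just a delay for one weapon type.
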(event `self.ReceiveBeginPlay`
  ;[0 0.03906 1 1 12] Reference to Player
  (bind _asbp_player (cast `/Game/FPSGame/Character/BP_Player` (`GameplayStatics.GetPlayerCharacter` 0)))
  (set `self.Player` _asbp_player))

(event `AutoReloadOnEmpty`
  ;[1 0 0.8203 1 12] Delay reloading so the last shot won't go astray
  (if (`|EnumEquality` (`self.WeaponType`) "NewEnumerator3")
    (`KismetSystemLibrary.Delay` 0.4)))

(fn `AmmoPickup`
  (params (AmmoType :type "/Game/FPSGame/Data/E_AmmoType Enum" :default "NewEnumerator0"))
  (returns (Success :type Boolean))
  (switch `/Game/FPSGame/Data/E_AmmoType` AmmoType
    (:`NewEnumerator0`
      ;[0.07812 1 0] Adds ammo if pistol is picking up pistol ammo
      (if (`|EnumEquality` (`self.WeaponType`) "NewEnumerator0")
        (set `self.CurrentTotalAmmo` (+ (`self.PistolPickupAmount`) (`self.CurrentTotalAmmo`)))
        (return true)
        (else
          (return false))))
    (:`NewEnumerator1`
      ;[0.07812 1 0] Adds ammo if pistol is picking up pistol ammo
      (if (`|EnumEquality` (`self.WeaponType`) "NewEnumerator1")
        (set `self.CurrentTotalAmmo` (+ (`self.RiflePickupAmount`) (`self.CurrentTotalAmmo`)))
        (return true)
        (else
          (return false))))
    (:`NewEnumerator2`
      ;[0.07812 1 0] Adds ammo if shotgun is picking up shotgun ammo
      (if (`|EnumEquality` (`self.WeaponType`) "NewEnumerator2")
        (set `self.CurrentTotalAmmo` (+ (`self.ShotgunPickupAmount`) (`self.CurrentTotalAmmo`)))
        (return true)
        (else
          (return false))))
    (:`NewEnumerator3`
      ;[0.07812 1 0] Adds ammo if sniper rifle is picking up sniper ammo
      (if (`|EnumEquality` (`self.WeaponType`) "NewEnumerator3")
        (set `self.CurrentTotalAmmo` (+ (`self.SniperPickupAmount`) (`self.CurrentTotalAmmo`)))
        (return true)
        (else
          (return false))))
    (:`NewEnumerator4`
      ;[0.07812 1 0] Adds ammo if grenade launcher is picking up grenade ammo
      (if (`|EnumEquality` (`self.WeaponType`) "NewEnumerator4")
        (set `self.CurrentTotalAmmo` (+ (`self.GrenadePickupAmount`) (`self.CurrentTotalAmmo`)))
        (return true)
        (else
          (return false))))
    (:`NewEnumerator5`
      ;[0.07812 1 0] Adds ammo if rocket launcher is picking up rocket ammo
      (if (`|EnumEquality` (`self.WeaponType`) "NewEnumerator5")
        (set `self.CurrentTotalAmmo` (+ (`self.RocketPickupAmount`) (`self.CurrentTotalAmmo`)))
        (return true)
        (else
          (return false))))))

(fn `CalculateLineTrace`
  (params (Camera :type "CameraComponent Object Reference") (WeaponMesh :type "SceneComponent Object Reference") (WeaponSocket :type Text))
  (returns (HitResult :type "HitResult Structure"))
  (locals (LocalCamera :type "CameraComponent Object Reference") (localWeaponSocket :type Text) (LocalWeaponMesh :type "SceneComponent Object Reference"))
  (bind _bulletspread (`self.BulletSpread`))
  (bind (_returnvalue_location _returnvalue_rotation) (`KismetMathLibrary.BreakTransform` (`SceneComponent.K2_GetComponentToWorld` (`local.LocalCamera`))))
  (bind _returnvalue (* _bulletspread -1.0))
  (bind _returnvalue_2 (+ _returnvalue_location (* (`KismetMathLibrary.GetForwardVector` _returnvalue_rotation) (`self.LineTraceDistance`))))
  (`|ExecutionSequence`
    (:`then_0`
      (set `local.LocalCamera` Camera))
    (:`then_1`
      (bind _outhit (`KismetSystemLibrary.LineTraceSingleForObjects` _returnvalue_location (select `bool` (`/Game/FPSGame/Character/BP_Player.IsAiming?` (`self.Player`)) :`false` (`KismetMathLibrary.MakeVector` (+ (.x _returnvalue_2) (`KismetMathLibrary.RandomFloatInRange` _returnvalue _bulletspread)) (+ (.y _returnvalue_2) (`KismetMathLibrary.RandomFloatInRange` _returnvalue _bulletspread)) (+ (.z _returnvalue_2) (`KismetMathLibrary.RandomFloatInRange` _returnvalue _bulletspread))) :`true` _returnvalue_2) (`|MakeArray` "ObjectTypeQuery1" "ObjectTypeQuery2" :!type "EObjectTypeQuery Enum") false (`|MakeArray` (`GameplayStatics.GetPlayerCharacter` 0) :!type "Actor Object Reference") "ForDuration" true (struct :`R` 1.0 :`A` 1.0) (struct :`G` 1.0 :`A` 1.0) 10.0)))))

(fn `DoWeHaveAmmo?`
  (returns (`HasAmmo?` :type Boolean))
  ;[0 1 0.7656 1 12] Allows shoot event to occur if player has ammo.
  (return (> (`self.CurrentAmmo`) 0)))

(fn `IsMagFullOrEmpty`
  (returns (ReturnValue :type Boolean))
  (if (== (`self.CurrentAmmo`) (`self.MagazineSize`))
    _
    (elif (== (`self.CurrentTotalAmmo`) 0)
      _
      (else
        ;[0.6867 0 1 1 12] Enables reload if mag is empty but ammo in reserves
        (bind _output_get (set `/Game/FPSGame/Character/BP_Player.CanReload?` true (`self.Player`)))
        (return _output_get))))
  ;[0.6867 0 1 1 12] Disables reload if mag is full or reserves are empty
  (bind _output_get_2 (set `/Game/FPSGame/Character/BP_Player.CanReload?` false (`self.Player`)))
  (return _output_get_2))

(fn `IsThereAmmoLeft?`
  (returns (ReturnValue :type Boolean))
  ;[0.6867 0 1 1 12] Check for ammo in reserve
  (return (> (`self.CurrentTotalAmmo`) 0)))

(fn `ReloadCalculation`
  (bind _output_get (set `self.BulletDifference` (- (`self.MagazineSize`) (`self.CurrentAmmo`))))
  (if (<= _output_get (`self.CurrentTotalAmmo`))
    ;[0.07399 0.1069 0.1719 1 12] Runs when there is reserve ammo
    (set `self.CurrentAmmo` (`self.MagazineSize`))
    (set `self.CurrentTotalAmmo` (- (`self.CurrentTotalAmmo`) (`self.BulletDifference`)))
    (else
      ;[0 0.1562 1 1 12] Runs when reserve amount is lower than the ammo in the magazine
      (set `self.CurrentAmmo` (+ (`self.CurrentAmmo`) (`self.CurrentTotalAmmo`)))
      (set `self.CurrentTotalAmmo` 0))))

(fn `StartShooting`
  (params (Firetype :type "/Game/FPSGame/Data/E-Firetype Enum" :default "NewEnumerator0"))
  (`|ExecutionSequence`
    (:`then_0`
      ;[1 0.3516 0 1 12] Subtracts a bullet when firing
      (set `self.CurrentAmmo` (- (`self.CurrentAmmo`) 1))
      ;[0 0.9766 1 1 12] Auto reload gun whem mag becomes empty
      (if (<= (`self.CurrentAmmo`) 0)
        (`self.AutoReloadOnEmpty`)))
    (:`then_1`
      (switch `/Game/FPSGame/Data/E-Firetype` Firetype
        (:`NewEnumerator0`
          (`self.CalculateLineTrace` (`/Game/FPSGame/Character/BP_Player.Camera` (`self.Player`)) (`self.WeaponMesh`) (`self.Weapon Socket`)))))))

(fn `UserConstructionScript`)