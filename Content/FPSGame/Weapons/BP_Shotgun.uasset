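; Shotgun weapon Blueprint that extends a parent weapon class's shooting behavior with shotgun-specific fire animations.
; StartShooting runs the parent logic, then plays the standard fire animation on the weapon mesh, or a no-cock variant when current ammo is zero.
; It then calls FireRateCalculate, and the construction script only defers to the parent.
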(event `self.StartShooting`
  (params (Firetype :type "/Game/FPSGame/Data/E-Firetype Enum" :default "NewEnumerator0"))
  (bind _weaponmesh (`self.WeaponMesh`))
  (`parent.StartShooting` Firetype)
  (if (not (== (`self.CurrentAmmo`) 0))
    (`SkeletalMeshComponent.PlayAnimation` _weaponmesh "/Game/WeaponMeshes/MilitaryWeapSilver/Weapons/Animations/Fire_Shotgun_W.Fire_Shotgun_W" false)
    (else
      (`SkeletalMeshComponent.PlayAnimation` _weaponmesh "/Game/WeaponMeshes/MilitaryWeapSilver/Weapons/Animations/Fire_ShotgunNOCock_W.Fire_ShotgunNOCock_W" false)))
  (`self.FireRateCalculate`))

(fn `UserConstructionScript`
  (`parent.UserConstructionScript`))