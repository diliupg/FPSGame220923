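; BP_WeaponPickupBase is a base weapon pickup actor that hands a weapon to the player when interacted with.
; BeginPlay caches the BP_Player reference, and InteractWithWeapon passes WeaponToSpawn to the player's WeaponPickup event.
; A DoOnce then plays the pickup sound and destroys the actor.
; Tick plays a timeline that adds local offsets to hover the pickup up and down.
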(event `self.ReceiveBeginPlay`
  ;[0.5703 0 1] Reference to Player
  (bind _asbp_player (cast `/Game/FPSGame/Character/BP_Player` (`GameplayStatics.GetPlayerCharacter` 0)))
  (set `self.Player` _asbp_player))

(event `InteractWithWeapon`
  ;[0 1 0.08594] Runs event in Bp_Player
  (`/Game/FPSGame/Character/BP_Player.WeaponPickup` (`self.Player`) (`self.WeaponToSpawn`))
  (`/Engine/EditorBlueprintResources/StandardMacros.DoOnce` false
    (:`Completed`
      (`GameplayStatics.PlaySound2D` (`self.PickupSound`) 1.0 1.0 0.0 null null)
      (`self.K2_DestroyActor`))))

(event `self.ReceiveTick`
  (params (DeltaSeconds :type "Float (single-precision)"))
  ;[0.5938 0 1] Hovers weapon up and down
  (bind (_direction _hoveranim) (`Timeline|BobUpAndDown`)
    (:`Update`
      (`self.K2_AddActorLocalOffset` _hoveranim))))

(fn `UserConstructionScript`)