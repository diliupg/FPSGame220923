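; First-person player character Blueprint handling movement, weapons, interaction, flashlight and HUD creation.
; Timelines drive a regenerating stamina sprint with exhaustion and a capsule-height crouch, while Tick selects head-bob camera shakes by speed.
; Picked-up weapons spawn attached to the arms across six key-bound slots, toggled by visibility behind a switch montage.
; Fire, reload and homing-missile toggle delegate to the current weapon; a camera line trace picks up weapons and ammo.
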(event `self.ReceiveBeginPlay`
  ;[1 0 0.3516 1 12] Get Capsule HalfHeight to variable
  (set `self.CapsuleHalfHeight` (`CapsuleComponent.CapsuleHalfHeight` (`self.CapsuleComponent`)))
  ;[1 0 0.1641 1 12] Creates main HUD
  (bind _returnvalue (`|CreateWidget` "/Game/FPSGame/UI/MainHUD.MainHUD_C"))
  (bind _output_get (set `self.MainHUD` _returnvalue))
  (`UserWidget.AddToViewport` _output_get 0))

(event `Fire`
  (bind _currentweapon (`self.CurrentWeapon`))
  (bind _currentweapon_2 (`self.CurrentWeapon`))
  (if (`self.CanShoot?`)
    (if (`/Game/FPSGame/Weapons/BP_WeaponBase.DoWeHaveAmmo?` _currentweapon_2)
      (`/Game/FPSGame/Weapons/BP_WeaponBase.StartShooting` _currentweapon (`/Game/FPSGame/Weapons/BP_WeaponBase.FireType` _currentweapon))
      (`KismetSystemLibrary.Delay` 0.2)
      (set `self.IsCockingShotgun?` true)
      ;[0.3594 1 0 1 12] Give time for the cocking animation to finish
      (`KismetSystemLibrary.Delay` 0.4)
      (set `self.IsCockingShotgun?` false)
      (elif (`/Game/FPSGame/Weapons/BP_WeaponBase.IsThereAmmoLeft?` _currentweapon_2)
        (`self.Reload`)
        (else
          (`GameplayStatics.PlaySound2D` "/Game/FPSGame/Audio/GunDryFire_Cue.GunDryFire_Cue" 1.0 1.0 0.0 null null))))))

(event `Reload`
  (bind _currentweapon (`self.CurrentWeapon`))
  (if (`self.CanWeReload?`)
    (`|ExecutionSequence`
      (:`then_0`
        (set `self.IsReloading?` true)
        (set `self.CanShoot?` false)
        (set `self.IsAiming?` false)
        (`KismetSystemLibrary.Delay` 0.5)
        (`|PlayMontage` (`self.PlayerArms`) (`/Game/FPSGame/Weapons/BP_WeaponBase.ReloadAnimMontage` (`self.CurrentWeapon`))
          (:`OnCompleted`
            (if (`self.IsReloading?`)
              (`/Game/FPSGame/Weapons/BP_WeaponBase.ReloadCalculation` (`self.CurrentWeapon`))
              (set `self.IsReloading?` false)
              (set `self.CanShoot?` true)))))
      (:`then_1`
        (if (not (`self.IsSprinting?`))
          (set `CharacterMovementComponent.MaxWalkSpeed` (`self.MaxWalkSpeed`) (`self.CharacterMovement`))))
      (:`then_2`
        (if (`/Game/FPSGame/Weapons/BP_WeaponBase.IsShotgun?` (`self.CurrentWeapon`))
          (`/Game/FPSGame/Weapons/BP_WeaponBase.ShotgunReloadPellets` _currentweapon)
          (`KismetSystemLibrary.Delay` (`/Game/FPSGame/Weapons/BP_WeaponBase.ReloadTime` _currentweapon))
          (set `/Game/FPSGame/Weapons/BP_WeaponBase.ReloadTime` 0.3 _currentweapon) ; Resetting back to default time
        )))))

(event `WeaponPickup`
  (params (WeaponToSpawn :type "/Game/FPSGame/Weapons/BP_WeaponBase Class Reference"))
  ;[1 0.6094 0 1 12] Weapon Pickup
  (bind _returnweapon (`self.SpawnWeapon` WeaponToSpawn))
  (`self.EquipWeapon` _returnweapon))

(event `EquipWeapon`
  (params (Weapon :type "/Game/FPSGame/Weapons/BP_WeaponBase Object Reference"))
  ;[0 1 0.25 1 12] EquipWeapon
  (if (not (`self.IsSwitchingWeapon?`))
    (if (`self.IsReloading?`)
      (set `self.IsReloading?` false))
    (set `self.IsSwitchingWeapon?` true)
    (`|PlayMontage` (`self.PlayerArms`) "/Game/MigratedAssets/FPSArms/Arms/Arms_Animations/Anim_Montages/Arms_Weapon_Down_Montage.Arms_Weapon_Down_Montage"
      (:`then`
        (`KismetSystemLibrary.Delay` 0.25)
        (`self.HideAndShowWeaponMesh` Weapon)
        (set `self.Loadout` "NewEnumerator1")
        ;;[0.007044 0 0.02083 1 12] Update Crosshair
        (`/Game/FPSGame/UI/CrossHairs.CrosshairUpdate` (`/Game/FPSGame/UI/MainHUD.CrossHairs` (`self.MainHUD`)))
        (set `self.IsSwitchingWeapon?` false)
        (set `self.CanShoot?` true) ; Can't shoot while switching weapon
      ))))

(event `HeadBob`
  (bind _returnvalue (`GameplayStatics.GetPlayerController` 0))
  (bind _returnvalue_2 (`KismetMathLibrary.VSize` (`self.GetVelocity`)))
  ;[0 0.7422 1 1 12] Player Headbob
  (if (and (> _returnvalue_2 0.0) (`self.CanJump`))
    (if (< _returnvalue_2 300.0)
      (`PlayerController.ClientStartCameraShake` :`self` _returnvalue :`Shake` "/Game/FPSGame/CameraMovement/WalkingCameraShake.WalkingCameraShake_C")
      (else
        (`PlayerController.ClientStartCameraShake` :`self` _returnvalue :`Shake` "/Game/FPSGame/CameraMovement/SprintingCameraShake.SprintingCameraShake_C")))
    (else
      (`PlayerController.ClientStartCameraShake` :`self` _returnvalue :`Shake` "/Game/FPSGame/CameraMovement/IdleCameraShake.IdleCameraShake_C"))))

(event `self.OnLanded`
  (params (Hit :type "HitResult Structure (by ref)"))
  ;[0 1 0.3906 1 12] Camera shake on JumpLand
  (`GameplayStatics.PlaySound2D` "/Game/FPSGame/Audio/Land.Land" 1.0 1.0 0.0 null null)
  (`GameplayStatics.PlayWorldCameraShake` "/Game/FPSGame/CameraMovement/JumpCameraShake.JumpCameraShake_C" (`self.K2_GetActorLocation`) 100.0 500.0))

(event `InputAction|HomingOn`
  (params (Key :type "Key Structure"))
  (bind _currentweapon (`self.CurrentWeapon`))
  ;[0.03992 0 0.04688 1 12] Homing Misslies On Off
  (:`Pressed`
    (if (`KismetSystemLibrary.IsValid` _currentweapon)
      (if (`|EnumEquality` (`/Game/FPSGame/Weapons/BP_WeaponBase.WeaponType` _currentweapon) "NewEnumerator5")
        (`/Engine/EditorBlueprintResources/StandardMacros.FlipFlop`
          (:`A`
            (set `/Game/FPSGame/Weapons/BP_WeaponBase.HomingMissile?` true _currentweapon))
          (:`B`
            (set `/Game/FPSGame/Weapons/BP_WeaponBase.HomingMissile?` false _currentweapon)))))))

(event `InputAction|Flashlight`
  (params (Key :type "Key Structure"))
  (bind _spotlight (`self.SpotLight`))
  ;[1 0.1172 0 1 12] Flashlight On Off
  (:`Pressed`
    ;;[0.02621 0.0141 0.1042 1 12] Comment
    (`GameplayStatics.PlaySound2D` "/Game/FPSGame/Audio/flashlight_on_off.flashlight_on_off" 0.15 1.0 0.0 null null)
    (`/Engine/EditorBlueprintResources/StandardMacros.FlipFlop`
      (:`A`
        (`SceneComponent.SetVisibility` _spotlight true false))
      (:`B`
        (`SceneComponent.SetVisibility` _spotlight false false)))))

(event `self.ReceiveTick`
  (params (DeltaSeconds :type "Float (single-precision)"))
  (`self.HeadBob`)
  ;[1 0.7031 0 1 12] Checks if W key is released while Sprinting
  (if (`self.HaveWeStoppedMoving?`)
    (`self.MovementStopped`) ; Connected to the Sprinting Timeline
  ))

(event `InputAxis|MoveForward`
  (params (AxisValue :type "Float (single-precision)"))
  ;[0 0.2219 1 1 12] WASD Movement Input
  (`self.AddMovementInput` (`KismetMathLibrary.GetForwardVector` (`KismetMathLibrary.MakeRotator` 0.0 0.0 (.yaw (`self.GetControlRotation`)))) AxisValue))

(event `InputAxis|MoveRight`
  (params (AxisValue :type "Float (single-precision)"))
  ;[0 0.2219 1 1 12] WASD Movement Input
  (`self.AddMovementInput` (`KismetMathLibrary.GetRightVector` (`KismetMathLibrary.MakeRotator` 0.0 0.0 (.yaw (`self.GetControlRotation`)))) AxisValue))

(event `InputAction|Jump`
  (params (Key :type "Key Structure"))
  ;[0 0.2219 1 1 12] Jump Action
  (:`Pressed`
    (`self.Jump`))
  (:`Released`
    (`self.StopJumping`)))

(event `InputAction|Sprint`
  (params (Key :type "Key Structure"))
  ;[0 1 0.6484 1 12] Sprint with regenerating Stamina Bar
  (:`Pressed`
    (if (not (`self.ISCrouching?`))
      (if (not (`self.IsAiming?`))
        (if (not (`self.IsReloading?`))
          (if (`self.AreWeExhausted?`)
            (`self.StartSprint`)
            (switch `/Game/FPSGame/Data/E_Loadout` (`self.Loadout`)
              (:`NewEnumerator0`
                (bind (_direction _staminaamount) (`Timeline|Timeline_0` :!label _label)
                  (:`Update`
                    (bind _output_get (set `self.EnergyLevel` _staminaamount)))
                  (:`Finished`
                    (if (== _output_get 0.0)
                      (`self.Exhausted`)))))
              (:`NewEnumerator1`
                (`/Game/FPSGame/Weapons/BP_WeaponBase.StopShooting` (`self.CurrentWeapon`))
                (goto _label)))))))))

(event `MovementStopped`
  ;[0 1 0.6484 1 12] Sprint with regenerating Stamina Bar
  (if (not (`self.IsExhausted?`))
    (`|ExecutionSequence`
      (:`then_0`
        (`self.StopSprint`)
        (goto _label :!via `Stop`))
      (:`then_1`
        (`KismetSystemLibrary.Delay` (`self.StaminaRegenPause`))
        (goto _label :!via `Reverse`)))))

(event `Exhausted`
  ;[0 1 0.6484 1 12] Sprint with regenerating Stamina Bar
  (set `self.IsExhausted?` true)
  (`self.StopSprint`)
  (`KismetSystemLibrary.Delay` (`self.ExhaustedTimer`)) ; Wait for some time before regenerating stamina
  (set `self.IsExhausted?` false)
  (goto _label :!via `ReverseFromEnd`))

(event `InputAction|Crouch`
  (params (Key :type "Key Structure"))
  ;[0 0.04248 0.1875 1 12] Initiate crouch
  (:`Pressed`
    (`self.StartCrouch`)
    (set `self.ISCrouching?` true)
    (bind (_direction _crouchalpha _camerarotationyaw _camerarotationpitch) (`Timeline|Timeline_1` :!label _label_2)
      (:`Update`
        (`CapsuleComponent.SetCapsuleHalfHeight` (`self.CapsuleComponent`) (`KismetMathLibrary.Lerp` (`self.CapsuleHalfHeight`) (`self.CapsuleCrouchHeight`) _crouchalpha) true)
        (`SceneComponent.K2_SetRelativeRotation` (`self.Camera`) (`KismetMathLibrary.MakeRotator` 0.0 _camerarotationpitch _camerarotationyaw) false false))))
  (:`Released`
    (`self.EndCrouch`)
    (set `self.ISCrouching?` false)))

(event `EndCrouch`
  ;[0 0.04248 0.1875 1 12] Activated when we release the Crouch button or if we press the Sprint button while Crouching
  (set `self.IsCrouching?` false)
  (set `CharacterMovementComponent.MaxWalkSpeed` (`self.MaxWalkSpeed`) (`self.CharacterMovement`))
  (goto _label_2 :!via `Reverse`))

(event `StartCrouch`
  (bind _charactermovement (`self.CharacterMovement`))
  ;[0 0.04248 0.1875 1 12] Crouch
  (if (not (`NavMovementComponent.IsFalling` (`self.CharacterMovement`)))
    (set `self.ISCrouching?` true)
    (`self.StopSprint`)
    (`self.MovementStopped`)
    (set `CharacterMovementComponent.MaxWalkSpeed` (`CharacterMovementComponent.MaxWalkSpeedCrouched` _charactermovement) _charactermovement)))

(event `Key|One`
  (params (Key :type "Key Structure"))
  (bind _weaponslot01 (`self.WeaponSlot01`))
  ;[0 0.9766 1 1 12] Key bindings to equip weappons after they have been initially picked up
  (:`Pressed`
    (if (`self.Is1stSlotFilled?`)
      (if (!= (`self.CurrentWeapon`) _weaponslot01)
        (`self.EquipWeapon` _weaponslot01)
        (set `self.CurrentWeapon` _weaponslot01)
        (`/Game/FPSGame/UI/CrossHairs.CrosshairUpdate` (`/Game/FPSGame/UI/MainHUD.CrossHairs` (`self.MainHUD`)) :!label _label)))))

(event `Key|Two`
  (params (Key :type "Key Structure"))
  (bind _weaponslot02 (`self.WeaponSlot02`))
  ;[0 0.9766 1 1 12] Key bindings to equip weappons after they have been initially picked up
  (:`Pressed`
    (if (`self.Is2ndSlotFilled?`)
      (if (!= (`self.CurrentWeapon`) _weaponslot02)
        (`self.EquipWeapon` _weaponslot02)
        (set `self.CurrentWeapon` _weaponslot02)
        (goto _label)))))

(event `Key|Three`
  (params (Key :type "Key Structure"))
  (bind _weaponslot03 (`self.WeaponSlot03`))
  ;[0 0.9766 1 1 12] Key bindings to equip weappons after they have been initially picked up
  (:`Pressed`
    (if (`self.Is3rdSlotFilled?`)
      (if (!= (`self.CurrentWeapon`) _weaponslot03)
        (`self.EquipWeapon` _weaponslot03)
        (set `self.CurrentWeapon` _weaponslot03)
        (goto _label)))))

(event `Key|Four`
  (params (Key :type "Key Structure"))
  (bind _weaponslot04 (`self.WeaponSlot04`))
  ;[0 0.9766 1 1 12] Key bindings to equip weappons after they have been initially picked up
  (:`Pressed`
    (if (`self.Is4thSlotFilled?`)
      (if (!= (`self.CurrentWeapon`) _weaponslot04)
        (`self.EquipWeapon` _weaponslot04)
        (set `self.CurrentWeapon` _weaponslot04)
        (goto _label)))))

(event `Key|Five`
  (params (Key :type "Key Structure"))
  (bind _weaponslot05 (`self.WeaponSlot05`))
  ;[0 0.9766 1 1 12] Key bindings to equip weappons after they have been initially picked up
  (:`Pressed`
    (if (`self.Is5thSlotFilled?`)
      (if (!= (`self.CurrentWeapon`) _weaponslot05)
        (`self.EquipWeapon` _weaponslot05)
        (set `self.CurrentWeapon` _weaponslot05)
        (goto _label)))))

(event `Key|Six`
  (params (Key :type "Key Structure"))
  (bind _weaponslot06 (`self.WeaponSlot06`))
  ;[0 0.9766 1 1 12] Key bindings to equip weappons after they have been initially picked up
  (:`Pressed`
    (if (`self.Is6thSlotFilled?`)
      (if (!= (`self.CurrentWeapon`) _weaponslot06)
        (`self.EquipWeapon` _weaponslot06)
        (set `self.CurrentWeapon` _weaponslot06)
        (goto _label)))))

(event `InputAction|Interact`
  (params (Key :type "Key Structure"))
  (bind _camera (`self.Camera`))
  (bind _returnvalue (`SceneComponent.K2_GetComponentLocation` _camera))
  ;[0.06771 0.009874 0.009874 1 12] Draws line trace to check if interacting with weapon or ammo
  (:`Pressed`
    (bind (_outhit _returnvalue_2) (`KismetSystemLibrary.LineTraceSingle` _returnvalue (+ _returnvalue (* (`SceneComponent.GetForwardVector` _camera) 200.0)) "TraceTypeQuery1"))
    (if _returnvalue_2
      (`|ExecutionSequence`
        (:`then_0`
          (switch `/Game/FPSGame/Data/E_Loadout` (`self.Loadout`) ; Can't grab ammo without weapon
            (:`NewEnumerator1`
              (bind (_bblockinghit _binitialoverlap _time _distance _location _impactpoint _normal _impactnormal _physmat _hitactor) (`GameplayStatics.BreakHitResult` _outhit))
              (bind _asammo_pickup_base (cast `/Game/FPSGame/Interactables/Ammo/AmmoPickupBase` _hitactor))
              (`/Game/FPSGame/Interactables/Ammo/AmmoPickupBase.PickupAmmo` _asammo_pickup_base))))
        (:`then_1`
          (bind _asbp_weapon_pickup_base (cast `/Game/FPSGame/Interactables/Weapons/BP_WeaponPickupBase` _hitactor))
          (`/Game/FPSGame/Interactables/Weapons/BP_WeaponPickupBase.InteractWithWeapon` _asbp_weapon_pickup_base))))))

(event `InputAction|Reload`
  (params (Key :type "Key Structure"))
  (:`Pressed`
    (switch `/Game/FPSGame/Data/E_Loadout` (`self.Loadout`)
      (:`NewEnumerator1`
        (bind _returnvalue (`/Game/FPSGame/Weapons/BP_WeaponBase.IsMagFullOrEmpty` (`self.CurrentWeapon`)))
        (if _returnvalue
          (if (`self.IsSprinting?`)
            (`self.MovementStopped`))
          ;[1 0.4002 0.1887 1 12] Stops gun from shooting while reloading
          (if (`/Game/FPSGame/Weapons/BP_WeaponBase.IsFiring?` (`self.CurrentWeapon`))
            (`/Game/FPSGame/Weapons/BP_WeaponBase.StopShooting` (`self.CurrentWeapon`)))
          (`self.Reload`))))))

(event `InputAction|Fire`
  (params (Key :type "Key Structure"))
  (:`Pressed`
    (switch `/Game/FPSGame/Data/E_Loadout` (`self.Loadout`)
      (:`NewEnumerator1`
        (if (not (`self.IsWeaponFireLoading?`))
          (if (`self.IsSprinting?`)
            (`self.MovementStopped`))
          (`self.Fire`)))))
  (:`Released`
    (switch `/Game/FPSGame/Data/E_Loadout` (`self.Loadout`)
      (:`NewEnumerator1`
        (`/Game/FPSGame/Weapons/BP_WeaponBase.StopShooting` (`self.CurrentWeapon`))))))

(fn `HideAndShowWeaponMesh`
  (params (Weapon :type "/Game/FPSGame/Weapons/BP_WeaponBase Object Reference"))
  (locals (LocalCurrentWeapon :type "/Game/FPSGame/Weapons/BP_WeaponBase Object Reference"))
  (bind _weaponslot05 (`self.WeaponSlot05`))
  (bind _weaponslot06 (`self.WeaponSlot06`))
  (bind _weaponslot01 (`self.WeaponSlot01`))
  (bind _weaponslot02 (`self.WeaponSlot02`))
  (bind _weaponslot03 (`self.WeaponSlot03`))
  (bind _weaponslot04 (`self.WeaponSlot04`))
  ;[0 0.2219 1] Hide currently used weapon slot
  (set `local.LocalCurrentWeapon` Weapon)
  (`/Engine/EditorBlueprintResources/StandardMacros.IsValid` _weaponslot01
    (:`Is Valid`
      (`self.SetActorHiddenInGame` _weaponslot01 true))
    (:`Is Not Valid`
      _))
  (`/Engine/EditorBlueprintResources/StandardMacros.IsValid` _weaponslot02
    (:`Is Valid`
      (`self.SetActorHiddenInGame` _weaponslot02 true))
    (:`Is Not Valid`
      _))
  (`/Engine/EditorBlueprintResources/StandardMacros.IsValid` _weaponslot03
    (:`Is Valid`
      (`self.SetActorHiddenInGame` _weaponslot03 true))
    (:`Is Not Valid`
      _))
  (`/Engine/EditorBlueprintResources/StandardMacros.IsValid` _weaponslot04
    (:`Is Valid`
      (`self.SetActorHiddenInGame` _weaponslot04 true))
    (:`Is Not Valid`
      _))
  (`/Engine/EditorBlueprintResources/StandardMacros.IsValid` _weaponslot05
    (:`Is Valid`
      (`self.SetActorHiddenInGame` _weaponslot05 true))
    (:`Is Not Valid`
      _))
  (`/Engine/EditorBlueprintResources/StandardMacros.IsValid` _weaponslot06
    (:`Is Valid`
      (`self.SetActorHiddenInGame` _weaponslot06 true))
    (:`Is Not Valid`
      _))
  ;[0 0.02543 0.1146] Shows currently equipped weapon mesh
  (if (== (`local.LocalCurrentWeapon`) (`self.WeaponSlot01`))
    (`self.SetActorHiddenInGame` (`self.WeaponSlot01`) false)
    (elif (== (`local.LocalCurrentWeapon`) (`self.WeaponSlot02`))
      (`self.SetActorHiddenInGame` (`self.WeaponSlot02`) false)
      (elif (== (`local.LocalCurrentWeapon`) (`self.WeaponSlot03`))
        (`self.SetActorHiddenInGame` (`self.WeaponSlot03`) false)
        (elif (== (`local.LocalCurrentWeapon`) (`self.WeaponSlot04`))
          (`self.SetActorHiddenInGame` (`self.WeaponSlot04`) false)
          (elif (== (`local.LocalCurrentWeapon`) (`self.WeaponSlot05`))
            (`self.SetActorHiddenInGame` (`self.WeaponSlot05`) false)
            (elif (== (`local.LocalCurrentWeapon`) (`self.WeaponSlot06`))
              (`self.SetActorHiddenInGame` (`self.WeaponSlot06`) false))))))))

(fn `SpawnWeapon`
  (params (Weapon :type "/Game/FPSGame/Weapons/BP_WeaponBase Class Reference"))
  (returns (ReturnWeapon :type "/Game/FPSGame/Weapons/BP_WeaponBase Object Reference"))
  (locals (LocalWeapon :type "/Game/FPSGame/Weapons/BP_WeaponBase Class Reference"))
  ;[0 0.2219 1 1 12] Spawns weapon actor in player's hands and assigns weapon slot
  (set `local.LocalWeapon` Weapon)
  (if (not (`self.Is1stSlotFilled?`))
    (bind _returnvalue (`|SpawnActorFromClass` (`local.LocalWeapon`) (`self.GetTransform`) "Undefined" "OverrideRootScale" null null))
    (bind _output_get (set `self.WeaponSlot01` _returnvalue))
    (set `self.Is1stSlotFilled?` true)
    (`self.K2_AttachToComponent` _output_get (`self.PlayerArms`) (`/Game/FPSGame/Weapons/BP_WeaponBase.SocketName` _returnvalue) "SnapToTarget" "SnapToTarget" "SnapToTarget" false)
    (bind _output_get_2 (set `self.CurrentWeapon` _output_get))
    (return _output_get_2)
    (elif (not (`self.Is2ndSlotFilled?`))
      (bind _returnvalue_2 (`|SpawnActorFromClass` (`local.LocalWeapon`) (`self.GetTransform`) "Undefined" "OverrideRootScale" null null))
      (bind _output_get_3 (set `self.WeaponSlot02` _returnvalue_2))
      (set `self.Is2ndSlotFilled?` true)
      (`self.K2_AttachToComponent` _output_get_3 (`self.PlayerArms`) (`/Game/FPSGame/Weapons/BP_WeaponBase.SocketName` _returnvalue_2) "SnapToTarget" "SnapToTarget" "SnapToTarget" false)
      (bind _output_get_4 (set `self.CurrentWeapon` _output_get_3))
      (return _output_get_4)
      (elif (not (`self.Is3rdSlotFilled?`))
        (bind _returnvalue_3 (`|SpawnActorFromClass` (`local.LocalWeapon`) (`self.GetTransform`) "Undefined" "OverrideRootScale" null null))
        (bind _output_get_5 (set `self.WeaponSlot03` _returnvalue_3))
        (set `self.Is3rdSlotFilled?` true)
        (`self.K2_AttachToComponent` _output_get_5 (`self.PlayerArms`) (`/Game/FPSGame/Weapons/BP_WeaponBase.SocketName` _returnvalue_3) "SnapToTarget" "SnapToTarget" "SnapToTarget" false)
        (bind _output_get_6 (set `self.CurrentWeapon` _output_get_5))
        (return _output_get_6)
        (elif (not (`self.Is4thSlotFilled?`))
          (bind _returnvalue_4 (`|SpawnActorFromClass` (`local.LocalWeapon`) (`self.GetTransform`) "Undefined" "OverrideRootScale" null null))
          (bind _output_get_7 (set `self.WeaponSlot04` _returnvalue_4))
          (set `self.Is4thSlotFilled?` true)
          (`self.K2_AttachToComponent` _output_get_7 (`self.PlayerArms`) (`/Game/FPSGame/Weapons/BP_WeaponBase.SocketName` _returnvalue_4) "SnapToTarget" "SnapToTarget" "SnapToTarget" false)
          (bind _output_get_8 (set `self.CurrentWeapon` _output_get_7))
          (return _output_get_8)
          (elif (not (`self.Is5thSlotFilled?`))
            (bind _returnvalue_5 (`|SpawnActorFromClass` (`local.LocalWeapon`) (`self.GetTransform`) "Undefined" "OverrideRootScale" null null))
            (bind _output_get_9 (set `self.WeaponSlot05` _returnvalue_5))
            (set `self.Is5thSlotFilled?` true)
            (`self.K2_AttachToComponent` _output_get_9 (`self.PlayerArms`) (`/Game/FPSGame/Weapons/BP_WeaponBase.SocketName` _returnvalue_5) "SnapToTarget" "SnapToTarget" "SnapToTarget" false)
            (bind _output_get_10 (set `self.CurrentWeapon` _output_get_9))
            (return _output_get_10)
            (elif (not (`self.Is6thSlotFilled?`))
              (bind _returnvalue_6 (`|SpawnActorFromClass` (`local.LocalWeapon`) (`self.GetTransform`) "Undefined" "OverrideRootScale" null null))
              (bind _output_get_11 (set `self.WeaponSlot06` _returnvalue_6))
              (set `self.Is6thSlotFilled?` true)
              (`self.K2_AttachToComponent` _output_get_11 (`self.PlayerArms`) (`/Game/FPSGame/Weapons/BP_WeaponBase.SocketName` _returnvalue_6) "SnapToTarget" "SnapToTarget" "SnapToTarget" false)
              (bind _output_get_12 (set `self.CurrentWeapon` _output_get_11))
              (return _output_get_12))))))))

(fn `StartSprint`
  (if (not (`NavMovementComponent.IsFalling` (`self.CharacterMovement`)))
    (set `CharacterMovementComponent.MaxWalkSpeed` (`self.SprintSpeed`) (`self.CharacterMovement`))
    (set `self.IsSprinting?` true)
    (set `self.ISCrouching?` false)))

(fn `StopSprint`
  (set `CharacterMovementComponent.MaxWalkSpeed` (`self.MaxWalkSpeed`) (`self.CharacterMovement`))
  (set `self.IsSprinting?` false))

(fn `UserConstructionScript`)